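; BP_player is a Paper2D player character that runs along one axis and jumps using Enhanced Input.
; BeginPlay adds the default mapping context through BP_PlayerController.
; Move input drives movement along actor forward, rotates the sprite to face travel, and switches run and idle flipbooks.
; Jumping blocks move input and plays a non-looping flipbook, then a delay loop polls for zero vertical velocity to restore idle.
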(event Input|EnhancedActionEvents|EnhancedInputActionIA_action
  (params (ActionValue :type Float%20%28double-precision%29) (ElapsedSeconds :type Float%20%28double-precision%29) (TriggeredSeconds :type Float%20%28double-precision%29) (InputAction :type Input%20Action%20Object%20Reference :default "/Game/Blueprint/IA_action.IA_action"))
  (:Triggered
    (if (not (Variables|Default|GetbisJumping))
      (Pawn|Input|AddMovementInput (Transformation|GetActorForwardVector) ActionValue false)
      (Sprite|SetFlipbook (Variables|Default|GetSprite) "/Game/Assets/FB_run.FB_run")
      (if (> ActionValue 0.0)
        (Transformation|SetWorldRotation (Variables|Default|GetSprite) "0, 0, 0" false false)
        (else
          (Transformation|SetWorldRotation (Variables|Default|GetSprite) "0.000000,180.000000,0.000000" false false)))))
  (:Completed
    (if (not (Variables|Default|GetbisJumping))
      (Sprite|SetFlipbook (Variables|Default|GetSprite) "/Game/Assets/FB_idle.FB_idle"))))

(event Input|EnhancedActionEvents|EnhancedInputActionIA_Jump
  (params (ActionValue :type Boolean) (ElapsedSeconds :type Float%20%28double-precision%29) (TriggeredSeconds :type Float%20%28double-precision%29) (InputAction :type Input%20Action%20Object%20Reference :default "/Game/Blueprint/IA_Jump.IA_Jump"))
  (bind _sprite (Variables|Default|GetSprite))
  (:Triggered
    (if (not (Variables|Default|GetbisJumping))
      (Variables|Default|SetbisJumping true)
      (Character|Jump)
      (Components|Timeline|SetLooping _sprite false)
      (Sprite|SetFlipbook _sprite "/Game/Assets/FB_jump.FB_jump")
      (Utilities|FlowControl|Delay 0.1)
      (if (== (.Z (Math|Vector|BreakVector (Transformation|GetVelocity))) 0.0) :!label _label
        (Components|Timeline|SetLooping _sprite true)
        (Audio|Components|Audio|Play _sprite)
        (Sprite|SetFlipbook _sprite "/Game/Assets/FB_idle.FB_idle")
        (Variables|Default|SetbisJumping false)
        (else
          (Utilities|FlowControl|Delay 0.1)
          (goto _label))))))

(event EventBeginPlay
  (bind _asbp_player_controller (Utilities|Casting|CastToBP_PlayerController (Pawn|GetController)))
  (Input|AddMappingContext (PlayerController|LocalPlayerSubsystems|GetEnhancedInputLocalPlayerSubsystem _asbp_player_controller) "/Game/Blueprint/IMC_default.IMC_default" 0 "(bIgnoreAllPressedKeysUntilRelease=True,bForceImmediately=False)"))

(fn ConstructionScript)